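; Colleague actor that players irritate by hitting it with throwables; filling its irritation meter makes it snap and wins the game.
; On overlap, HitCollision accepts each throwable once, and GetHit adds its clamped irritation value, records noise level and location, and updates the player's HUD.
; It also plays a gendered 2D sound, selected by the colleague's StressToy variable rather than the incoming throwable.
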(event `self.ReceiveBeginPlay`
  (`KismetSystemLibrary.Delay` 0.2)
  (bind _returnvalue (`GameplayStatics.GetActorOfClass` "/Game/OfficeMayhem/Blueprints/Player/BP_Player.BP_Player_C"))
  (`/Engine/EditorBlueprintResources/StandardMacros.IsValid` _returnvalue
    (:`Is Valid`
      (bind _hudref (`/Game/OfficeMayhem/Blueprints/Player/BP_Player.HUDRef` _returnvalue))
      (`/Engine/EditorBlueprintResources/StandardMacros.IsValid` _hudref
        (:`Is Valid`
          (bind _output_get (set `self.HUDRef` _hudref))
          (`/Game/OfficeMayhem/UI/WBP_OfficeHUD.UpdateIrritation` _output_get (`self.CurrentIrritation`) (`self.MaxIrritation`)))))))

(event `self.HitCollision.OnComponentBeginOverlap`
  (params (OverlappedComponent :type "PrimitiveComponent Object Reference") (OtherActor :type "Actor Object Reference") (OtherComp :type "PrimitiveComponent Object Reference") (OtherBodyIndex :type Integer) (bFromSweep :type Boolean) (SweepResult :type "HitResult Structure (by ref)"))
  (bind _asbp_throwable_base (cast `/Game/OfficeMayhem/Blueprints/Throwables/BP_ThrowableBase` OtherActor))
  (if (not (`/Game/OfficeMayhem/Blueprints/Throwables/BP_ThrowableBase.HasHit` _asbp_throwable_base))
    (set `/Game/OfficeMayhem/Blueprints/Throwables/BP_ThrowableBase.HasHit` true _asbp_throwable_base)
    (`self.GetHit` _asbp_throwable_base)))

(fn `GetHit`
  (params (Throwable :type "/Game/OfficeMayhem/Blueprints/Throwables/BP_ThrowableBase Object Reference"))
  (bind _throwable (`local.Throwable`))
  (bind _output_get (set `self.CurrentIrritation` (`KismetMathLibrary.FClamp` (+ (`self.CurrentIrritation`) (`/Game/OfficeMayhem/Blueprints/Throwables/BP_ThrowableBase.IrritationValue` Throwable)) 0.0 (`self.MaxIrritation`))))
  (`/Game/OfficeMayhem/UI/WBP_OfficeHUD.UpdateIrritation` (`self.HUDRef`) _output_get (`self.MaxIrritation`))
  (if (>= _output_get (`self.MaxIrritation`))
    (`self.Snap`)
    (else
      (set `self.ColleagueState` "NewEnumerator1")))
  (set `self.LastNoiseLevel` (`/Game/OfficeMayhem/Blueprints/Throwables/BP_ThrowableBase.NoiseLevel` _throwable))
  (set `self.LastImpactLocation` (`self.K2_GetActorLocation` _throwable))
  (if (`self.IsMale?`)
    (switch `/Game/OfficeMayhem/Blueprints/Throwables/E_OfficeObjectType` "NewEnumerator4"
      (:`NewEnumerator0`
        (`GameplayStatics.PlaySound2D` "/Game/OfficeMayhem/SFX/Male/PaperballMale.PaperballMale" 1.0 1.0 0.0 null null))
      (:`NewEnumerator1`
        (`GameplayStatics.PlaySound2D` "/Game/OfficeMayhem/SFX/Male/PaperclipMale.PaperclipMale" 1.0 1.0 0.0 null null))
      (:`NewEnumerator2`
        (`GameplayStatics.PlaySound2D` "/Game/OfficeMayhem/SFX/Male/SpongeMale.SpongeMale" 1.0 1.0 0.0 null null))
      (:`NewEnumerator3`
        (`GameplayStatics.PlaySound2D` "/Game/OfficeMayhem/SFX/Male/CoffeeCupMale.CoffeeCupMale" 1.0 1.0 0.0 null null))
      (:`NewEnumerator4`
        (`GameplayStatics.PlaySound2D` "/Game/OfficeMayhem/SFX/Male/StressToyMale.StressToyMale" 1.0 1.0 0.0 null null))
      (:`NewEnumerator5`
        (`GameplayStatics.PlaySound2D` "/Game/OfficeMayhem/SFX/Male/StaplerMale.StaplerMale" 1.0 1.0 0.0 null null)))
    (else
      (switch `/Game/OfficeMayhem/Blueprints/Throwables/E_OfficeObjectType` "NewEnumerator4"
        (:`NewEnumerator0`
          (`GameplayStatics.PlaySound2D` "/Game/OfficeMayhem/SFX/Female/PaperballFemale.PaperballFemale" 1.0 1.0 0.0 null null))
        (:`NewEnumerator1`
          (`GameplayStatics.PlaySound2D` "/Game/OfficeMayhem/SFX/Female/PaperclipFemale.PaperclipFemale" 1.0 1.0 0.0 null null))
        (:`NewEnumerator2`
          (`GameplayStatics.PlaySound2D` "/Game/OfficeMayhem/SFX/Female/SpongeFemale.SpongeFemale" 1.0 1.0 0.0 null null))
        (:`NewEnumerator3`
          (`GameplayStatics.PlaySound2D` "/Game/OfficeMayhem/SFX/Female/CoffeeCupFemale.CoffeeCupFemale" 1.0 1.0 0.0 null null))
        (:`NewEnumerator4`
          (`GameplayStatics.PlaySound2D` "/Game/OfficeMayhem/SFX/Female/StressToyFemale.StressToyFemale" 1.0 1.0 0.0 null null))
        (:`NewEnumerator5`
          (`GameplayStatics.PlaySound2D` "/Game/OfficeMayhem/SFX/Female/StaplerFemale.StaplerFemale" 1.0 1.0 0.0 null null))))))

(fn `Snap`
  (set `self.ColleagueState` "NewEnumerator4")
  (bind _asgm_office_mayhem (cast `/Game/OfficeMayhem/Blueprints/GM_OfficeMayhem` (`GameplayStatics.GetGameMode`)))
  (`/Game/OfficeMayhem/Blueprints/GM_OfficeMayhem.WinGame` _asgm_office_mayhem))

(fn `UserConstructionScript`)