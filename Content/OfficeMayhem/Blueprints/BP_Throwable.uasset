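; BP_Throwable is a physics-driven thrown object whose look and weight come from a data table.
; On BeginPlay it looks up its RowName in DT_Throwables, sets the mesh and mass, and destroys itself if the row is missing.
; It then ignores its owner when moving, enables physics simulation and launches at InitialVelocity.
; A fixed lifespan removes it afterwards.
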(event `self.ReceiveBeginPlay`
  (bind _mesh (`self.Mesh`))
  (bind _returnvalue (`|GetDataTableRow` "/Game/OfficeMayhem/Blueprints/DT_Throwables.DT_Throwables" (`self.RowName`))
    (:`then`
      (bind _output_get (set `self.Stats` _returnvalue))
      (bind (_displayname _mesh_2 _weight) (break `/Game/OfficeMayhem/Blueprints/S_ThrowableStats` _output_get))
      (`StaticMeshComponent.SetStaticMesh` _mesh _mesh_2)
      (`PrimitiveComponent.SetMassOverrideInKg` _mesh "None" _weight true)
      (`PrimitiveComponent.IgnoreActorWhenMoving` _mesh (`self.GetOwner`) true)
      (`PrimitiveComponent.SetSimulatePhysics` _mesh true)
      (`PrimitiveComponent.SetPhysicsLinearVelocity` _mesh (`self.InitialVelocity`) false "None")
      (`self.SetLifeSpan` 15.0))
    (:`RowNotFound`
      (`self.K2_DestroyActor`))))

(fn `UserConstructionScript`)