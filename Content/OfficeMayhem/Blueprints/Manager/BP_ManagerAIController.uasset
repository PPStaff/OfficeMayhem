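; AI controller for the manager character, providing a patrol step along the points stored on BP_Manager.
; MoveToNextPatrolPoint issues a move to the current point, then advances the pawn's patrol index.
; On wrap-around it calls itself immediately, so the move to the first point replaces the one to the last.
; The event graph's only call to it is unreachable, and BeginPlay and Tick are empty.
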(event `self.ReceiveBeginPlay`)

(fn `MoveToNextPatrolPoint`
  (bind _asbp_manager (cast `/Game/OfficeMayhem/Blueprints/Manager/BP_Manager` (`self.K2_GetPawn`)))
  (bind _patrolpoints (`/Game/OfficeMayhem/Blueprints/Manager/BP_Manager.PatrolPoints` _asbp_manager))
  (`self.MoveToActor` (`|GetArrayItem` _patrolpoints (`/Game/OfficeMayhem/Blueprints/Manager/BP_Manager.PatrolIndex` _asbp_manager)) 50.0 true true true null)
  (bind _patrolindex (`/Game/OfficeMayhem/Blueprints/Manager/BP_Manager.PatrolIndex` _asbp_manager))
  (set `/Game/OfficeMayhem/Blueprints/Manager/BP_Manager.PatrolIndex` (+ _patrolindex 1) _asbp_manager)
  (if (>= _patrolindex (`KismetArrayLibrary.Array_Length` _patrolpoints))
    (set `/Game/OfficeMayhem/Blueprints/Manager/BP_Manager.PatrolIndex` 0 _asbp_manager)
    (`self.MoveToNextPatrolPoint`)))

(fn `UserConstructionScript`)