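; BP_Manager is the office manager character in Office Mayhem that spots the player and ends the game when suspicion maxes out.
; On BeginPlay it slows its walk and moves to a random patrol point, then once more after a random wait, without looping.
; When the player enters DetectionSphere, a Visibility line trace confirms sight and adds suspicion once, more if charging.
; Full suspicion triggers a one-time LoseGame call on GM_OfficeMayhem.
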(event `self.ReceiveBeginPlay`
  (set `CharacterMovementComponent.MaxWalkSpeed` 250.0 (`self.CharacterMovement`))
  (`self.MoveToRandomPatrolPoint`)
  (`KismetSystemLibrary.Delay` (`KismetMathLibrary.RandomFloatInRange` (`self.MinWaitTime`) (`self.MaxWaitTime`)))
  (`self.MoveToRandomPatrolPoint`))

(event `self.DetectionSphere.OnComponentBeginOverlap`
  (params (OverlappedComponent :type "PrimitiveComponent Object Reference") (OtherActor :type "Actor Object Reference") (OtherComp :type "PrimitiveComponent Object Reference") (OtherBodyIndex :type Integer) (bFromSweep :type Boolean) (SweepResult :type "HitResult Structure (by ref)"))
  (bind _asbp_player (cast `/Game/OfficeMayhem/Blueprints/Player/BP_Player` OtherActor))
  (if (`/Game/OfficeMayhem/Blueprints/Player/BP_Player.IsCharging` _asbp_player)
    (bind _cansee (`self.CanSeePlayer` _asbp_player))
    (if _cansee
      (`self.AddSuspicion` 10.0))
    (else
      (bind _cansee_2 (`self.CanSeePlayer` _asbp_player))
      (if _cansee_2
        (`self.AddSuspicion` 5.0)))))

(fn `AddSuspicion`
  (params (Amount :type "Float (double-precision)"))
  (bind _output_get (set `self.Suspicion` (`KismetMathLibrary.FClamp` (+ (`self.Suspicion`) Amount) 0.0 (`self.MaxSuspicion`))))
  (if (>= _output_get (`self.MaxSuspicion`))
    (`self.CatchPlayer`)))

(fn `CanSeePlayer`
  (params (PlayerActor :type "Actor Object Reference"))
  (returns (CanSee :type Boolean))
  (bind _outhit (`KismetSystemLibrary.LineTraceSingle` :`Start` (+ (`self.K2_GetActorLocation` self) (`KismetMathLibrary.MakeVector` 0.0 0.0 150.0)) :`End` (+ (`self.K2_GetActorLocation` PlayerActor) (`KismetMathLibrary.MakeVector` 0.0 0.0 80.0)) :`TraceChannel` "TraceTypeQuery1" :`DrawDebugType` "ForDuration"))
  (return (== (`.HitActor` (`GameplayStatics.BreakHitResult` _outhit)) (`local.PlayerActor`))))

(fn `CatchPlayer`
  (if (not (`self.PlayerCaught`))
    (set `self.PlayerCaught` true)
    (bind _asgm_office_mayhem (cast `/Game/OfficeMayhem/Blueprints/GM_OfficeMayhem` (`GameplayStatics.GetGameMode`)))
    (`/Game/OfficeMayhem/Blueprints/GM_OfficeMayhem.LoseGame` _asgm_office_mayhem)))

(fn `MoveToRandomPatrolPoint`
  (bind _returnvalue (`KismetArrayLibrary.Array_Length` (`self.PatrolPoints`)))
  (if (> _returnvalue 0)
    (`AIBlueprintHelperLibrary.SimpleMoveToActor` (`self.GetController`) (`|GetArrayItem` (`self.PatrolPoints`) (`KismetMathLibrary.RandomIntegerInRange` 0 (- _returnvalue 1))))))

(fn `UserConstructionScript`)